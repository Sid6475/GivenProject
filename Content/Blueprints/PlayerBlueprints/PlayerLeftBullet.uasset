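; Player projectile, named as the left-side bullet, that kills ground and air AI enemies on overlap.
; A timeline started at BeginPlay moves it without sweep by adding a track offset to the location cached in the construction script.
; Overlapping an enemy destroys it with a type-specific death sound.
; The bullet spawns an explosion and destroys itself on enemy overlap, on any hit, or when Tick finds the timeline exactly at 1.5 seconds.
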(event `self.ReceiveBeginPlay`
  ;[1 1 1] Moves the bullet right when it enters the world.
  (bind (_direction _newtrack_0) (`Timeline|LeftBulletTimeline`)
    (:`Update`
      (`self.K2_SetActorLocation` (+ (`self.StartLocation`) _newtrack_0)))))

(event `self.ReceiveTick`
  (params (DeltaSeconds :type "Float (single-precision)"))
  ;[1 1 1] Destroys the bullet when it finishes the timeline. (1.5 seconds)
  (if (== (`TimelineComponent.GetPlaybackPosition` (`self.LeftBulletTimeline`)) 1.5)
    (`|SpawnActorFromClass` "/Game/Blueprints/PlayerBlueprints/BulletExplosion.BulletExplosion_C" (`self.GetTransform`) "Undefined" "OverrideRootScale" null null)
    (`self.K2_DestroyActor`)))

(event `self.ReceiveActorBeginOverlap`
  (params (OtherActor :type "Actor Object Reference"))
  ;[1 1 1] If the bullet hits an enemy, destroy the enemy and the bullet.
  (bind _asbp_ground_ai (cast `/Game/Blueprints/AiBlueprints/BP_GroundAi` OtherActor)
    (:`then`
      (`self.K2_DestroyActor` _asbp_ground_ai)
      (`GameplayStatics.PlaySound2D` "/Game/Audio/GameAudio/AiAudio/GroundEnemyDeath.GroundEnemyDeath" 1.0 1.0 0.0 null null))
    (:`CastFailed`
      (bind _asbp_air_ai (cast `/Game/Blueprints/AiBlueprints/BP_AirAi` OtherActor))
      (`self.K2_DestroyActor` _asbp_air_ai)
      (`GameplayStatics.PlaySound2D` "/Game/Audio/GameAudio/AiAudio/AirEnemyDeath.AirEnemyDeath" 1.0 1.0 0.0 null null)))
  (`|SpawnActorFromClass` "/Game/Blueprints/PlayerBlueprints/BulletExplosion.BulletExplosion_C" (`self.GetTransform`) "Undefined" "OverrideRootScale" null null)
  (`self.K2_DestroyActor`))

(event `self.ReceiveHit`
  (params (MyComp :type "PrimitiveComponent Object Reference") (Other :type "Actor Object Reference") (OtherComp :type "PrimitiveComponent Object Reference") (bSelfMoved :type Boolean) (HitLocation :type "Vector Structure") (HitNormal :type "Vector Structure") (NormalImpulse :type "Vector Structure") (Hit :type "HitResult Structure (by ref)"))
  ;[1 1 1] Destroys the bullet when it hits something.
  (`|SpawnActorFromClass` "/Game/Blueprints/PlayerBlueprints/BulletExplosion.BulletExplosion_C" (`self.GetTransform`) "Undefined" "OverrideRootScale" null null)
  (`self.K2_DestroyActor`))

(fn `UserConstructionScript`
  (bind _returnvalue (`self.K2_GetActorLocation`))
  (`self.K2_SetActorLocation` _returnvalue)
  (set `self.StartLocation` _returnvalue))