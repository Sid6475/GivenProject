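; BP_GroundAi is a sprite-based ground enemy that patrols back and forth and explodes when shot.
; A timeline started on BeginPlay offsets it from the StartLocation saved in the construction script, moving it without sweep.
; Tick sets FacingRight from the timeline's playback position and flips the sprite through negative X scale.
; A capsule overlap with BP_Bullet swaps in the BulletExplosion flipbook, then destroys the actor after a short delay.
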(event `self.ReceiveTick`
  (params (DeltaSeconds :type "Float (single-precision)"))
  ;[1 1 1] This is used to flip the sprite when it starts moving in the other direction
  (`self.Tick1`)
  (`self.Tick2`))

(event `self.ReceiveBeginPlay`
  ;[1 1 1] Makes Ai move back and forth
  (bind (_direction _newtrack_0) (`Timeline|GroundAiTimeline`)
    (:`Update`
      (`self.K2_SetActorLocation` (+ (`self.StartLocation`) _newtrack_0)))))

(event `Tick1`
  ;[1 1 1] This is used to flip the sprite when it starts moving in the other direction
  (if (`self.FacingRight`)
    (`self.SetActorScale3D` (0.35 0.35 0.35))
    (else
      (`self.SetActorScale3D` (-0.35 0.35 0.35)))))

(event `Tick2`
  ;[1 1 1] This is used to flip the sprite when it starts moving in the other direction
  (if (>= (`TimelineComponent.GetPlaybackPosition` (`self.GroundAiTimeline`)) 10.0)
    (set `self.FacingRight` false)
    (else
      (set `self.FacingRight` true))))

(event `self.Capsule.OnComponentBeginOverlap`
  (params (OverlappedComponent :type "PrimitiveComponent Object Reference") (OtherActor :type "Actor Object Reference") (OtherComp :type "PrimitiveComponent Object Reference") (OtherBodyIndex :type Integer) (bFromSweep :type Boolean) (SweepResult :type "HitResult Structure (by ref)"))
  (cast `/Game/2DSideScrollerBP/Blueprints/BP_Bullet` OtherActor)
  (`PaperFlipbookComponent.SetFlipbook` (`self.RenderComponent`) "/Game/Sprites/BulletExplosion/BulletExplosion.BulletExplosion")
  ;[1 1 1] This is used to flip the sprite when it starts moving in the other direction
  (`KismetSystemLibrary.Delay` 1.0)
  (`self.K2_DestroyActor`))

(fn `UserConstructionScript`
  (bind _returnvalue (`self.K2_GetActorLocation`))
  (`self.K2_SetActorLocation` _returnvalue)
  (set `self.StartLocation` _returnvalue))