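; Teleporter actor that moves any overlapping actor to the location of a linked Destination actor.
; On overlap, it checks and clears the Destination's CanTeleport flag, teleports the actor with zeroed rotation and plays a 2D sound.
; A three-second delay then re-enables the flag as a cooldown.
; The Destination validity check runs only after its flag is read and cleared.
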(event `self.ReceiveActorBeginOverlap`
  (params (OtherActor :type "Actor Object Reference"))
  (bind _destination (`self.Destination`))
  ;[1 1 1] Teleport Function
  (if (`/Game/Blueprints/Platforms_Teleporters/TeleportToOne.CanTeleport` (`self.Destination`))
    (set `/Game/Blueprints/Platforms_Teleporters/TeleportToOne.CanTeleport` false _destination)
    (`/Engine/EditorBlueprintResources/StandardMacros.IsValid` _destination
      (:`Is Valid`
        (`self.K2_TeleportTo` :`self` OtherActor :`DestLocation` (`self.K2_GetActorLocation` _destination))
        (`GameplayStatics.PlaySound2D` "/Game/Audio/GameAudio/SFX/Teleport.Teleport" 1.0 1.0 0.0 null null)
        (`KismetSystemLibrary.Delay` 3.0)
        (set `/Game/Blueprints/Platforms_Teleporters/TeleportToOne.CanTeleport` true (`self.Destination`))))))

(fn `UserConstructionScript`)